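; BP_EnemySpawner is a queue-based spawn point for the enemy waves system, spawning enemies at its own transform.
; AddEnemyToQueue queues an enemy type and spawns immediately unless the sphere overlaps that type.
; After the game state's level-start event, a looping timer retries SpawnEnemy every couple of seconds without checking overlaps.
; SpawnEnemy uses the passed class rather than the queued entry, then removes the queue's first element.
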(event Custom|TryToSpawnEnemy
  ;[1 1 1] Not the best solution but makes not a big deal for performance
  (CallFunction|SpawnEnemy (Variables|Default|GetEnemyType)))

(event Custom|ActivateSpawner
  ;[1 1 1] Not the best solution but makes not a big deal for performance
  (Utilities|Time|SetTimerbyEvent (delegate Custom|TryToSpawnEnemy) 2.0 true))

(event EventBeginPlay
  ;[1 1 1] Not the best solution but makes not a big deal for performance
  (EventDispatchers|BindEventtoOnLevelStart (.AsThird%20Person%20Game%20State (Utilities|Casting|CastToThirdPersonGameState (Game|GetGameState))) (delegate Custom|ActivateSpawner)))

(fn ConstructionScript)

(fn SpawnEnemy
  (params (EnemyType :type Enemy%20Base%20Class%20Reference))
  (if (Utilities|Array|IsValidIndex (Variables|Default|GetEnemyQueue))
    (Game|SpawnActorfromClass EnemyType (Transformation|GetActorTransform) "AdjustIfPossibleButAlwaysSpawn" "MultiplyWithRoot" 0 0)
    (Utilities|Array|RemoveIndex (Variables|Default|GetEnemyQueue))
    (return true)
    (else
      (return false))))

(fn AddEnemytoQueue
  (params (EnemyType :type Enemy%20Base%20Class%20Reference%20%28by%20ref%29))
  (Utilities|Array|Add (Variables|Default|GetEnemyQueue) EnemyType)
  (if (Utilities|Array|IsValidIndex (Collision|GetOverlappingActors (Variables|Default|GetSphere) EnemyType :!class /Script/Engine.PrimitiveComponent))
    (Development|PrintString "ENEMY COLLIDES WITH OTHER" true true "(R=1.000000,G=0.141812,B=0.000000,A=1.000000)")
    (else
      (CallFunction|SpawnEnemy EnemyType))))