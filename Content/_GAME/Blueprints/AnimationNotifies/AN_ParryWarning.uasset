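; Animation notify state that shows a parry warning on ranged enemies during a marked window of an animation.
; On begin and end, it gets the enemy from the mesh owner through an interface message and casts it to BP_Enemy_Ranged.
; It makes that enemy's ParryWarningWidget visible at begin and hides it at end, doing nothing if the cast fails.
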(fn ReceivedNotifyBegin
  (params (MeshComp :type Skeletal%20Mesh%20Component%20Object%20Reference) (Animation :type Anim%20Sequence%20Base%20Object%20Reference) (TotalDuration :type Float%20%28single-precision%29) (EventReference :type Anim%20Notify%20Event%20Reference%20Structure%20%28by%20ref%29))
  (bind _enemyreference (Class|EnemyInterface|GetEnemyReference(Message) (Components|GetOwner MeshComp)))
  (bind _asbp_enemy_ranged (Utilities|Casting|CastToBP_Enemy_Ranged _enemyreference))
  (Rendering|SetVisibility (Variables|/Game/_GAME/Blueprints/Characters/Enemy/Blueprints/BP_Enemy_Ranged.BP_Enemy_Ranged_C|GetParryWarningWidget _asbp_enemy_ranged) true false)
  (return false))

(fn ReceivedNotifyEnd
  (params (MeshComp :type Skeletal%20Mesh%20Component%20Object%20Reference) (Animation :type Anim%20Sequence%20Base%20Object%20Reference) (EventReference :type Anim%20Notify%20Event%20Reference%20Structure%20%28by%20ref%29))
  (bind _enemyreference (Class|EnemyInterface|GetEnemyReference(Message) (Components|GetOwner MeshComp)))
  (bind _asbp_enemy_ranged (Utilities|Casting|CastToBP_Enemy_Ranged _enemyreference))
  (Rendering|SetVisibility (Variables|/Game/_GAME/Blueprints/Characters/Enemy/Blueprints/BP_Enemy_Ranged.BP_Enemy_Ranged_C|GetParryWarningWidget _asbp_enemy_ranged) false false)
  (return false))