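; Ranged enemy character that spawns a rifle on BeginPlay, attaches it to its hand socket and reports a fixed attack and defend range.
; Attacks chain a pre-shoot montage into a shoot montage, whose notify triggers a debug-drawn line trace from the AI's target back to the weapon.
; A damageable hit on another team takes fixed damage, tagged Melee despite being a shot.
; Completing the shoot montage signals attack end.
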(event EventBeginPlay
  (|CallParentFunction)
  (Class|EnemyInterface|EquipWeapon))

(event EventEquipWeapon
  (bind _returnvalue (Game|SpawnActorfromClass "/Game/_GAME/Blueprints/ItemBlueprints/EnemyWeapons/BP_EnemyWeapon_Rifle.BP_EnemyWeapon_Rifle_C" (Transformation|GetActorTransform) "Undefined" "MultiplyWithRoot" 0 0))
  (bind _output_get (Variables|Default|SetWeaponActor _returnvalue))
  (Transformation|AttachComponentToComponent _output_get (Variables|Character|GetMesh) "middle_01_r_rifle_socket" "SnapToTarget" "SnapToTarget" "SnapToTarget" true))

(event EventDefaultAttack
  (params (AttackTarget :type Actor%20Object%20Reference))
  (|CallParentFunction AttackTarget)
  (Animation|Montage|PlayMontage (Variables|Character|GetMesh) "/Game/_GAME/Blueprints/Characters/Enemy/Animations/Montages/MM_Enemy_Ranged_Preshoot_Montage.MM_Enemy_Ranged_Preshoot_Montage" 1.25
    (:OnCompleted
      (bind _notifyname (Animation|Montage|PlayMontage (Variables|Character|GetMesh) "/Game/_GAME/Blueprints/Characters/Enemy/Animations/Montages/MM_Enemy_Ranged_Shoot_Montage.MM_Enemy_Ranged_Shoot_Montage")
        (:OnCompleted
          (Default|CallOnAttackEndEvent))
        (:OnNotifyBegin
          (switch name _notifyname
            (:Fire
              (bind _aicontroller (Variables|Default|GetAIController)
                (:then
                  (bind _attacktarget (Variables|/Game/_GAME/Blueprints/Characters/Enemy/Blueprints/AI/AIC_Enemy.AIC_Enemy_C|GetAttackTarget _aicontroller)
                    (:then
                      (bind (_outhit _returnvalue) (Collision|LineTraceForObjects (Transformation|GetActorLocation _attacktarget) (Transformation|GetActorLocation (Variables|Default|GetWeaponActor)) (Utilities|Array|MakeArray "ObjectTypeQuery1" "ObjectTypeQuery3" "ObjectTypeQuery2") false 0 "ForDuration"))
                      (if _returnvalue
                        (if (Utilities|DoesObjectImplementInterface (.HitActor (Collision|BreakHitResult _outhit)) "/Script/CuttingEdge.IDamagable")
                          (bind _idamagable (Class|IDamagable|GetDamagableReference(Message) (.HitActor (Collision|BreakHitResult _outhit))))
                          (bind _teamnumber (Class|IDamagable|GetTeamNumber _idamagable))
                          (bind _teamnumber_2 (Class|IDamagable|GetTeamNumber self))
                          (if (!= _teamnumber_2 _teamnumber)
                            (bind _idamagable_2 (Class|IDamagable|GetDamagableReference(Message) (.HitActor (Collision|BreakHitResult _outhit))))
                            (Class|IDamagable|TakeDamage _idamagable_2 (Utilities|Struct|MakeDamageInfo 5.0 "Melee" "HitReaction" false true true) self)))))
                    (:else)))
                (:else)))))))))

(fn ConstructionScript
  (|CallParentFunction))

(fn GetIdealRangetoAttack
  (return 6e+02 6e+02))