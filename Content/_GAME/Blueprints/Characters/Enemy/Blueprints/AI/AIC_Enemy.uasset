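; AI controller for enemies that runs the possessed BP_Enemy_Base's behaviour tree and drives its blackboard state.
; On possess it sets Passive and copies the pawn's attack and defend radii into the blackboard.
; Sight or damage perception of an actor on another team switches a passive enemy to Attacking.
; Helper functions set Passive, Attacking, Staggered or Dead, falling back to Passive if the attack target is invalid or dead.
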(event OnPerceptionUpdated(AIPerception)
  (params (UpdatedActors :type Array%20of%20Actor%20Object%20References))
  (for _array_element UpdatedActors
    (Utilities|FlowControl|Sequence
      (:then_0
        (bind _sensed (CallFunction|CanSenseActor _array_element "NewEnumerator1"))
        (if _sensed
          (CallFunction|HandleSensedSight _array_element)))
      (:then_1
        (bind _sensed_2 (CallFunction|CanSenseActor _array_element "NewEnumerator2"))
        (if _sensed_2
          (CallFunction|HandleSensedDamage _array_element))))))

(event EventPossess
  (params (PossessedPawn :type Pawn%20Object%20Reference))
  (bind _asbp_enemy_base (Utilities|Casting|CastToBP_Enemy_Base PossessedPawn))
  (bind _behaviourtree (Variables|/Game/_GAME/Blueprints/Characters/Enemy/Blueprints/BP_Enemy_Base.BP_Enemy_Base_C|GetBehaviourTree _asbp_enemy_base)
    (:then
      (AI|RunBehaviorTree _behaviourtree)
      (CallFunction|SetStateasPassive)
      (bind (_attackradius _defendradius) (Class|EnemyInterface|GetIdealRangetoAttack(Message) PossessedPawn))
      (AI|Components|Blackboard|SetValueasFloat (Variables|Default|GetBlackboard) (Variables|Default|GetAttackRadiusKeyName) _attackradius)
      (AI|Components|Blackboard|SetValueasFloat (Variables|Default|GetBlackboard) (Variables|Default|GetDefendRadiusKeyName) _defendradius))
    (:else
      (Development|PrintString "NO VALID TREE ON ENEMY" true true "(R=1.000000,G=0.701072,B=0.000000,A=1.000000)"))))

(fn ConstructionScript)

(fn SetStateasPassive
  (AI|Components|Blackboard|SetValueasEnum (Variables|Default|GetBlackboard) (Variables|Default|GetStateKeyName) (Utilities|Enum|LiteralenumENUM_AIStates "NewEnumerator0")))

(fn SetStateasStaggered
  (AI|Components|Blackboard|SetValueasEnum (Variables|Default|GetBlackboard) (Variables|Default|GetStateKeyName) (Utilities|Enum|LiteralenumENUM_AIStates "NewEnumerator2")))

(fn SetStateasAttacking
  (params (InputAttackTarget :type Actor%20Object%20Reference) (UseLastKnownAttackTarget :type Boolean))
  (bind _output_get (LocalVariables|SetNewAttackTarget (select (and UseLastKnownAttackTarget (Utilities|IsValid (Variables|Default|GetAttackTarget))) (Variables|Default|GetAttackTarget) InputAttackTarget)))
  (Utilities|IsValid _output_get
    (:Is%20Valid
      (bind _isdead (Class|IDamagable|IsDead(Message) _output_get))
      (if _isdead
        (CallFunction|SetStateasPassive :!label _label)
        (else
          (AI|Components|Blackboard|SetValueasObject (Variables|Default|GetBlackboard) (Variables|Default|GetAttackTargetKeyName) _output_get)
          (AI|Components|Blackboard|SetValueasEnum (Variables|Default|GetBlackboard) (Variables|Default|GetStateKeyName) (Utilities|Enum|LiteralenumENUM_AIStates "NewEnumerator1"))
          (Variables|Default|SetAttackTarget (LocalVariables|GetNewAttackTarget)))))
    (:Is%20Not%20Valid
      (goto _label))))

(fn SetStateasDead
  (AI|Components|Blackboard|SetValueasEnum (Variables|Default|GetBlackboard) (Variables|Default|GetStateKeyName) (Utilities|Enum|LiteralenumENUM_AIStates "NewEnumerator3")))

(fn CanSenseActor
  (params (Actor :type Actor%20Object%20Reference) (Sense :type ENUM_AISenses%20Enum :default "NewEnumerator0"))
  (bind _info (Class|AIPerceptionComponent|GetActorsPerception (Variables|Default|GetAIPerception) Actor))
  (for _array_element (.LastSensedStimuli (Utilities|Struct|BreakActorPerceptionBlueprintInfo _info))
    (bind _returnvalue (Class|AIPerceptionSystem|GetSenseClassforStimulus _array_element))
    (if (== _returnvalue (Utilities|Select :Index Sense :NewEnumerator0 0 :NewEnumerator1 "/Script/AIModule.AISense_Sight" :NewEnumerator2 "/Script/AIModule.AISense_Damage"))
      (return _array_element (.bSuccessfullySensed (Utilities|Struct|BreakAIStimulus _array_element))))))

(fn HandleSensedSight
  (params (Actor :type Actor%20Object%20Reference))
  (bind _currentstate (CallFunction|GetCurrentState))
  (bind _sameteam (CallFunction|OntheSameTeam Actor))
  (if (not _sameteam)
    (switch Utilities|FlowControl|Switch|SwitchonENUM_AIStates _currentstate
      (:NewEnumerator0
        (CallFunction|SetStateasAttacking Actor false)))))

(fn GetCurrentState
  (return (Utilities|Enum|ByteToEnumENUM_AIStates (Class|BlackboardComponent|GetValueasEnum (Variables|Default|GetBlackboard) (Variables|Default|GetStateKeyName)))))

(fn HandleSensedDamage
  (params (Actor :type Actor%20Object%20Reference))
  (bind _currentstate (CallFunction|GetCurrentState))
  (bind _sameteam (CallFunction|OntheSameTeam Actor))
  (if (not _sameteam)
    (switch Utilities|FlowControl|Switch|SwitchonENUM_AIStates _currentstate
      (:NewEnumerator0
        (CallFunction|SetStateasAttacking Actor false)))))

(fn OntheSameTeam
  (params (Other :type Actor%20Object%20Reference))
  (bind _teamnumber (Class|IDamagable|GetTeamNumber(Message) Other))
  (bind _teamnumber_2 (Class|IDamagable|GetTeamNumber(Message) (Pawn|GetControlledPawn)))
  (return (== _teamnumber_2 _teamnumber)))