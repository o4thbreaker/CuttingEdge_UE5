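; Melee enemy child Blueprint that spawns a sword onto a hand socket and attacks with a combo montage.
; Light attacks sphere-trace between blade sockets, damaging pawns of other teams and using a hit array, cleared when the montage ends, to prevent repeat hits.
; Incoming damage goes through DamageSystem after a random block roll for blockable hits, but block events are empty, with their logic disconnected and marked for a shield enemy type.
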(event Custom|StartBlocking
  ;[1 0 0.2455] Block logic segment (MOVE TO SHIELD ENEMY TYPE)
)

(event Custom|EndBlocking
  ;[1 0 0.2455] Block logic segment (MOVE TO SHIELD ENEMY TYPE)
)

(event EventBeginPlay
  (|CallParentFunction))

(event EventDamageResponse
  (params (DamageResponse :type EDamageResponse%20Enum :default "None") (DamageDealer :type Actor%20Object%20Reference))
  ;[1 1 1] Damage response
  (|CallParentFunction DamageResponse DamageDealer))

(event EventEquipWeapon
  ;[1 1 1] Equip sword
  (bind _returnvalue (Game|SpawnActorfromClass "/Game/_GAME/Blueprints/ItemBlueprints/EnemyWeapons/BP_EnemyWeapon_Sword.BP_EnemyWeapon_Sword_C" (Transformation|GetActorTransform) "Undefined" "MultiplyWithRoot" 0 0))
  (bind _output_get (Variables|Default|SetWeaponActor _returnvalue))
  (Transformation|AttachComponentToComponent _output_get (Variables|Character|GetMesh) "enemy_sword_socket" "SnapToTarget" "SnapToTarget" "SnapToTarget" true)
  (Variables|Default|SetIsWieldingWeapon true))

(event EventDefaultAttack
  (params (AttackTarget :type Actor%20Object%20Reference))
  ;[1 1 1] Default attack
  (|CallParentFunction AttackTarget)
  (Animation|Montage|PlayMontage (Variables|Character|GetMesh) "/Game/_GAME/Blueprints/Characters/Enemy/Animations/Montages/AM_Enemy_Melee_Attack_ComboA1.AM_Enemy_Melee_Attack_ComboA1"
    (:OnCompleted
      _)
    (:OnInterrupted
      _))
  (Utilities|Array|Clear (Variables|Default|GetTempHitArray))
  (Class|EnemyInterface|AttackEnd AttackTarget))

(event EventBlocked
  (params (CanBeParried :type Boolean) (DamageDealer :type Actor%20Object%20Reference))
  ;[1 0 0.2455] Block logic segment (MOVE TO SHIELD ENEMY TYPE)
)

(event EventDeath
  ;[1 1 1] Death
  (|CallParentFunction))

(fn ConstructionScript
  (|CallParentFunction))

(fn TrytoBlock
  (if (<= (Math|Random|RandomFloat) (LocalVariables|GetBlockChance))
    (CallFunction|StartBlocking)))

(fn TakeDamage
  (params (DamageInfo :type Damage%20Info%20Structure) (DamageCauser :type Actor%20Object%20Reference))
  (if (.CanBeBlocked (Utilities|Struct|BreakDamageInfo DamageInfo))
    (CallFunction|TrytoBlock))
  (bind _wasdamaged (Class|DamageSystem|TakeDamage (Variables|Default|GetDamageSystem) DamageInfo DamageCauser))
  (return _wasdamaged))

(fn IsDead
  (return (Variables|/Script/CuttingEdge.DamageSystem|GetIsDead (Variables|Default|GetDamageSystem))))

(fn AttackDetection
  (params (WeaponRadius :type Float%20%28double-precision%29) (DamageInfo :type Damage%20Info%20Structure) (HitParticle :type Particle%20System%20Object%20Reference) (SwingSound :type Sound%20Base%20Object%20Reference) (Weapon :type Scene%20Component%20Object%20Reference))
  (bind (_outhit _returnvalue) (Collision|SphereTraceForObjects (Transformation|GetSocketLocation Weapon "BladeStart") (Transformation|GetSocketLocation Weapon "BladeEnd") WeaponRadius (Utilities|Array|MakeArray "ObjectTypeQuery3") false 0 "None"))
  (if _returnvalue
    (bind _teamnumber (Class|IDamagable|GetTeamNumber(Message) (.HitActor (Collision|BreakHitResult _outhit))))
    (bind _teamnumber_2 (Class|IDamagable|GetTeamNumber(Message) self))
    (if (and (not (Utilities|Array|ContainsItem (Variables|Default|GetTempHitArray) (.HitActor (Collision|BreakHitResult _outhit)))) (!= _teamnumber_2 _teamnumber))
      (bind _output_get (LocalVariables|SetActorToDamage (.HitActor (Collision|BreakHitResult _outhit))))
      (bind _wasdamaged (Class|IDamagable|TakeDamage(Message) _output_get DamageInfo self))
      (Utilities|Array|AddUnique (Variables|Default|GetTempHitArray) (LocalVariables|GetActorToDamage))
      (if _wasdamaged
        _
        (else
          _))
      (return _wasdamaged (LocalVariables|GetActorToDamage)))))

(fn PerformLightAttack
  (CallFunction|AttackDetection 15.0 (Utilities|Struct|MakeDamageInfo 1.0 "Melee" "HitReaction" false true true) 0 0 (Variables|/Script/Engine.Actor|GetRootComponent (Variables|Default|GetWeaponActor)))
  (return true))