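; Base enemy character Blueprint that links combat reactions to AIC_Enemy state changes and exposes references such as its patrol route.
; On spawn and death it notifies the GameState; death also unpossesses the controller, plays a montage and despawns the enemy with its weapon.
; When hit, it turns to the attacker and staggers, choosing hit reactions from a map keyed by the player's current montage.
; It returns to attacking when the reaction completes or is interrupted.
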(event EventBeginPlay
  ;[1 1 1] Set default values
  (|CallParentFunction)
  (bind _asaic_enemy (Utilities|Casting|CastToAIC_Enemy (AI|GetAIController self))
    (:then
      (Variables|Default|SetAIController _asaic_enemy)
      (Collision|SetCollisionResponsetoChannel (Variables|Default|GetCapsuleComponent) "ECC_Camera" "ECR_Ignore")
      (Utilities|FlowControl|DelayUntilNextTick)
      (Class|IEventManager|CallEnemySpawn(Message) (Game|GetGameState)))
    (:CastFailed
      (Development|PrintString "CAST TO AI FAILED" true true "(R=1.000000,G=0.000000,B=0.031298,A=1.000000)"))))

(event EventBlocked
  (params (CanBeParried :type Boolean) (DamageDealer :type Actor%20Object%20Reference))
  ;[1 1 1] Blocked
  (Development|PrintString "ENEMY_BASE BLOCKED" true true "(R=0.000000,G=1.000000,B=0.293706,A=1.000000)"))

(event EventDamageResponse
  (params (DamageResponse :type EDamageResponse%20Enum :default "None") (DamageDealer :type Actor%20Object%20Reference))
  ;[1 1 1] Reaction to getting hit
  (|CallParentFunction DamageResponse DamageDealer)
  (bind _playerreference (Class|BPIPlayer|GetPlayerReference(Message) DamageDealer))
  (Class|CombatSystem|RotatetoTargetActor (Variables|Default|GetCombatSystem) DamageDealer)
  (Default|SetStateasStaggered (Variables|Default|GetAIController))
  (Animation|Montage|PlayMontage (Variables|Character|GetMesh) (Utilities|Select :Index DamageResponse :None "/Game/_GAME/Blueprints/Characters/Enemy/Animations/Montages/AM_Shield_Hit_Left.AM_Shield_Hit_Left" :HitReaction (.Value (Utilities|Map|Find (Variables|Default|GetMontages) (Animation|GetCurrentMontage _playerreference :!class /Script/Engine.Character))) :Stagger 0 :Stun 0 :Knockback 0) (Variables|Default|GetHitReactionPlayRate)
    (:OnCompleted
      _)
    (:OnInterrupted
      _))
  (bind _teamnumber (Class|IDamagable|GetTeamNumber(Message) DamageDealer))
  (Utilities|FlowControl|DelayUntilNextTick)
  (Default|SetStateasAttacking (Variables|Default|GetAIController) (select (!= _teamnumber 0) DamageDealer 0) true))

(event EventDeath
  (bind _aicontroller (Variables|Default|GetAIController))
  ;[1 1 1] Death
  (Class|IEventManager|CallEnemyDeath(Message) (Game|GetGameState))
  (Default|SetStateasDead _aicontroller)
  (Class|EnemyInterface|LockOffThisActor)
  (Pawn|UnPossess _aicontroller)
  (|CallParentFunction)
  (Animation|Montage|PlayMontage (Variables|Character|GetMesh) "/Game/_GAME/Assets/Animations/AnimationMontages/AM_Death.AM_Death"
    (:then
      (Utilities|FlowControl|Delay 5.0)
      (CallFunction|DespawnEnemy))))

(fn ConstructionScript
  (Variables|Default|Set_FrontArrow (Variables|Default|GetFrontArrow))
  (Variables|Default|Set_BackArrow (Variables|Default|GetBackArrow))
  (Variables|Default|Set_LeftArrow (Variables|Default|GetLeftArrow))
  (Variables|Default|Set_RightArrow (Variables|Default|GetRightArrow)))

(fn DespawnEnemy
  (Utilities|FlowControl|Sequence
    (:then_0
      (bind _weaponactor (Variables|Default|GetWeaponActor)
        (:then
          (Actor|DestroyActor _weaponactor)
          (Variables|Default|SetWeaponActor 0))
        (:else)))
    (:then_1
      (Actor|DestroyActor))))

(fn GetDamagableReference
  (return self))

(fn GetPatrolRoute
  (return (Variables|AI|GetPatrolRoute)))

(fn GetEnemyReference
  (return self))